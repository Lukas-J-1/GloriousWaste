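; BP_PlankWall is a breakable wall built from five static mesh planks that breaks when something overlaps its box collision.
; On overlap it destroys the collision box so the break fires only once.
; It then spawns a BP_Plank actor at each mesh's world location and rotation and hides that static mesh, swapping static planks for separate actors.
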(event `self.BoxCollision.OnComponentBeginOverlap`
  (params (OverlappedComponent :type "PrimitiveComponent Object Reference") (OtherActor :type "Actor Object Reference") (OtherComp :type "PrimitiveComponent Object Reference") (OtherBodyIndex :type Integer) (bFromSweep :type Boolean) (SweepResult :type "HitResult Structure (by ref)"))
  (`ActorComponent.K2_DestroyComponent` (`self.BoxCollision`))
  (for _array_element (`|MakeArray` (`self.PlankStaticMesh1`) (`self.PlankStaticMesh2`) (`self.PlankStaticMesh3`) (`self.PlankStaticMesh4`) (`self.PlankStaticMesh5`) :!type "SceneComponent Object Reference")
    (`|SpawnActorFromClass` "/Game/Blueprints/Movable/BP_Plank.BP_Plank_C" (`KismetMathLibrary.MakeTransform` (`SceneComponent.K2_GetComponentLocation` _array_element) (`SceneComponent.K2_GetComponentRotation` _array_element)) "Undefined" "MultiplyWithRoot" null null)
    (`SceneComponent.SetVisibility` _array_element false false)))

(fn `UserConstructionScript`)